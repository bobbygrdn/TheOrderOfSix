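; Base item actor that shows an equip prompt when the player character overlaps it.
; On begin overlap it flags the TheOrderOfSix character as overlapping an item, creates an EquipPrompt widget, passes it to SetCorrectItemName and adds it to the viewport.
; On end overlap it clears the flag and removes every top-level EquipPrompt widget.
; SetCorrectItemName is empty here.
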(event `self.ReceiveActorBeginOverlap`
  (params (OtherActor :type "Actor Object Reference"))
  (bind _asthe_order_of_six_character (cast `TheOrderOfSixCharacter` OtherActor))
  (set `TheOrderOfSixCharacter.isOverlappingItem` true _asthe_order_of_six_character)
  (bind _returnvalue (`|CreateWidget` "/Game/Blueprints/EquipPrompt.EquipPrompt_C"))
  (`self.SetCorrectItemName` _returnvalue)
  (`UserWidget.AddToViewport` _returnvalue 0))

(event `self.ReceiveActorEndOverlap`
  (params (OtherActor :type "Actor Object Reference"))
  (bind _asthe_order_of_six_character (cast `TheOrderOfSixCharacter` OtherActor))
  (set `TheOrderOfSixCharacter.isOverlappingItem` false _asthe_order_of_six_character)
  (bind _foundwidgets (`WidgetBlueprintLibrary.GetAllWidgetsOfClass` "/Game/Blueprints/EquipPrompt.EquipPrompt_C"))
  (for _array_element _foundwidgets
    (`Widget.RemoveFromParent` _array_element)))

(fn `SetCorrectItemName`
  (params (WidgetReference :type "/Game/Blueprints/EquipPrompt Object Reference")))

(fn `UserConstructionScript`)