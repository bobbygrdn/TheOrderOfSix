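; Base enemy Blueprint with a health bar widget component that shows only when something is nearby.
; On BeginPlay it casts the widget to EnemyHealthBar and sets itself as that widget's owner.
; Overlap begin and end events on the ShowHealthBarVolume component toggle the health bar's visibility, with no filter on the overlapping actor.
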(event `self.ReceiveBeginPlay`
  (bind _asenemy_health_bar (cast `/Game/Blueprints/Widgets/EnemyHealthBar` (`WidgetComponent.GetUserWidgetObject` (`self.HealthBar`))))
  (set `/Game/Blueprints/Widgets/EnemyHealthBar.HealthBarOwner` self _asenemy_health_bar))

(event `self.ShowHealthBarVolume.OnComponentBeginOverlap`
  (params (OverlappedComponent :type "PrimitiveComponent Object Reference") (OtherActor :type "Actor Object Reference") (OtherComp :type "PrimitiveComponent Object Reference") (OtherBodyIndex :type Integer) (bFromSweep :type Boolean) (SweepResult :type "HitResult Structure (by ref)"))
  (`SceneComponent.SetVisibility` (`self.HealthBar`) true false))

(event `self.ShowHealthBarVolume.OnComponentEndOverlap`
  (params (OverlappedComponent :type "PrimitiveComponent Object Reference") (OtherActor :type "Actor Object Reference") (OtherComp :type "PrimitiveComponent Object Reference") (OtherBodyIndex :type Integer))
  (`SceneComponent.SetVisibility` (`self.HealthBar`) false false))

(fn `UserConstructionScript`)